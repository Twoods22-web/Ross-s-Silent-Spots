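; Moving platform actor that shuttles endlessly between its starting location and an offset position, starting at BeginPlay.
; A single Timeline adds its Alpha output to the cached start location each update, moving the actor without sweep.
; When the Timeline finishes, it waits through a fixed delay, then checks its direction to play in reverse or forward again.
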(event Custom|moveplatform
  (bind (_direction _alpha) (Timeline|Timeline PlayFromStart)
    (:Update
      (Transformation|SetActorLocation (+ (Variables|Default|GetStartLocation) _alpha) false false))
    (:Finished
      (Utilities|FlowControl|Delay 1e+01)
      (switch Utilities|FlowControl|Switch|SwitchonETimelineDirection _direction
        (:Forward
          (CallFunction|Moveplatformtostartlocation))
        (:Backward
          (CallFunction|Moveplatform))))))

(event Custom|moveplatformtostartlocation
  (bind (_direction _alpha) (Timeline|Timeline ReverseFromEnd)
    (:Update
      (Transformation|SetActorLocation (+ (Variables|Default|GetStartLocation) _alpha) false false))
    (:Finished
      (Utilities|FlowControl|Delay 1e+01)
      (switch Utilities|FlowControl|Switch|SwitchonETimelineDirection _direction
        (:Forward
          (CallFunction|Moveplatformtostartlocation))
        (:Backward
          (CallFunction|Moveplatform))))))

(event EventBeginPlay
  (Variables|Default|SetStartLocation (Transformation|GetActorLocation))
  (CallFunction|Moveplatform))

(fn ConstructionScript)